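; BP_Asteroid is an environment asteroid actor that varies its look each time play begins.
; On BeginPlay it gives the Asteroid component a random uniform scale, clamped to a fixed range, and a random rotation on all three axes.
; The randomization is unseeded and runs only at runtime, as the construction script is empty and there is no per-frame movement logic.
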(event `self.ReceiveBeginPlay`
  ; Randomize start rotation
  (`SceneComponent.SetRelativeScale3D` (`self.Asteroid`) (`KismetMathLibrary.Conv_DoubleToVector` (`KismetMathLibrary.FClamp` (* (`KismetMathLibrary.RandomFloat`) 3.0) 0.33 2.0)))
  (`SceneComponent.K2_SetRelativeRotation` (`self.Asteroid`) (`KismetMathLibrary.MakeRotator` (* (`KismetMathLibrary.RandomFloat`) 360.0) (* (`KismetMathLibrary.RandomFloat`) 360.0) (* (`KismetMathLibrary.RandomFloat`) 360.0)) false false))

(fn `UserConstructionScript`)